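; BP_Enemy is an enemy ship Blueprint that handles randomized coloring, spawn-in scaling and explosion effects.
; SetColor picks random body and wing colors from four-option palettes, applies them through a dynamic instance of M_Base_Ship and stores both.
; It then plays a timeline that drives actor scale.
; SpawnExplosion spawns PS_Explosion at the ship's location, passing the stored colors as emitter parameters.
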(event EventBeginPlay)

(event Collision|EventActorBeginOverlap
  (params (OtherActor :type Actor%20Object%20Reference)))

(event EventTick
  (params (DeltaSeconds :type Float%20%28single-precision%29)))

(event EventSetColor
  (Variables|Default|SetBodyColorIndex (Math|Random|RandomIntegerinRange 0 3))
  (Variables|Default|SetWingColorIndex (Math|Random|RandomIntegerinRange 0 3))
  (bind _returnvalue (Rendering|Material|CreateDynamicMaterialInstance "/Game/SpaceshipBattle/Materials/M_Base_Ship.M_Base_Ship" "None" "None" :!class /Script/Engine.KismetMaterialLibrary))
  (Rendering|Material|SetVectorParameterValue _returnvalue "Color1" (Utilities|Select :Index (Variables|Default|GetBodyColorIndex) :Option%200 "(R=0.124271,G=0.966667,B=0.132856,A=1.000000)" :Option%201 "(R=0.253784,G=0.202342,B=0.904167,A=1.000000)" :Option%202 "(R=0.954167,G=0.081108,B=0.073515,A=1.000000)" :Option%203 "(R=0.899856,G=0.925000,B=0.111997,A=1.000000)") :!class /Script/Engine.MaterialInstanceDynamic)
  (Variables|Default|SetPrimaryColor (Utilities|Select :Index (Variables|Default|GetBodyColorIndex) :Option%200 "(R=0.124271,G=0.966667,B=0.132856,A=1.000000)" :Option%201 "(R=0.253784,G=0.202342,B=0.904167,A=1.000000)" :Option%202 "(R=0.954167,G=0.081108,B=0.073515,A=1.000000)" :Option%203 "(R=0.899856,G=0.925000,B=0.111997,A=1.000000)"))
  (Rendering|Material|SetVectorParameterValue _returnvalue "Color2" (Utilities|Select :Index (Variables|Default|GetWingColorIndex) :Option%200 "(R=0.746190,G=0.163065,B=0.887500,A=1.000000)" :Option%201 "(R=0.000000,G=0.000000,B=0.000000,A=1.000000)" :Option%202 "(R=1.000000,G=0.576275,B=0.058333,A=1.000000)" :Option%203 "(R=0.233230,G=0.824163,B=0.858333,A=1.000000)") :!class /Script/Engine.MaterialInstanceDynamic)
  (Rendering|Material|SetMaterial (Variables|Default|GetShipSM) 0 _returnvalue)
  (Variables|Default|SetSecondryColor (Utilities|Select :Index (Variables|Default|GetWingColorIndex) :Option%200 "(R=0.746190,G=0.163065,B=0.887500,A=1.000000)" :Option%201 "(R=0.000000,G=0.000000,B=0.000000,A=1.000000)" :Option%202 "(R=1.000000,G=0.576275,B=0.058333,A=1.000000)" :Option%203 "(R=0.233230,G=0.824163,B=0.858333,A=1.000000)"))
  (bind _scale (Timeline|SpawnScaleTimeline Play)
    (:Update
      (Transformation|SetActorScale3D (Math|Conversions|ToVector(Float) _scale)))))

(event EventSpawnExplosion
  (bind _returnvalue (Effects|SpawnEmitteratLocation "/Game/ParticleSystem/PS_Explosion.PS_Explosion" (Transformation|GetActorLocation)))
  (Effects|Components|ParticleSystem|SetColorParameter _returnvalue "PrimaryColor" (Variables|Default|GetPrimaryColor))
  (Effects|Components|ParticleSystem|SetColorParameter _returnvalue "SecondyColor" (Variables|Default|GetSecondryColor)))

(fn ConstructionScript)